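; Player character Blueprint that fades objects blocking the view between its camera and spring arm.
; Each Tick, a helper runs a Visibility line trace from the camera to the spring arm.
; When hit time is below a threshold, it prints the hit actor's mesh component name and sets that mesh's Opacity material parameter.
; Opacity is never restored here, and DisableAllInput is an empty stub.
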(event EventTick
  (params (DeltaSeconds :type Float%20%28single-precision%29))
  (bind (_outhit_time _outhit_hitactor) (|LineTrace (Transformation|GetWorldLocation (Variables|Default|GetCamera)) (Transformation|GetWorldLocation (Variables|Default|GetSpringArm))))
  (if (< _outhit_time (Variables|CameraView|GetThreshold%20NotSee%20Camera))
    (Development|PrintString (Utilities|GetDisplayName (Actor|GetComponentbyClass _outhit_hitactor "/Script/Engine.MeshComponent")))
    (Rendering|Material|SetScalarParameterValueonMaterials (Actor|GetComponentbyClass _outhit_hitactor "/Script/Engine.MeshComponent") "Opacity" (Variables|CameraView|GetOpacity%20To%20set))))

(fn ConstructionScript)

(fn DisableAllInput)