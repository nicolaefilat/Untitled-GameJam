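; Dog AI character that catches the player and restarts the game.
; Capsule overlaps with the third-person character start or clear a catch timer, only while the AI controller's blackboard reports line of sight.
; Tick watches the timer and, past TimeToCatch, disables player input, shows a widget and restarts through the GameMode after a delay.
; UpdateWalkSpeed sets the movement component's maximum walk speed.
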(event OnComponentBeginOverlap(Capsule)
  (params (OverlappedComponent :type Primitive%20Component%20Object%20Reference) (OtherActor :type Actor%20Object%20Reference) (OtherComp :type Primitive%20Component%20Object%20Reference) (OtherBodyIndex :type Integer) (bFromSweep :type Boolean) (SweepResult :type Hit%20Result%20Structure%20%28by%20ref%29))
  (Utilities|Casting|CastToBP_ThirdPersonCharacter OtherActor)
  (if (ScalableFloat|GetValueasBool (Variables|/Script/AIModule.AIController|GetBlackboard (Variables|Default|GetAs%20Dog%20AI%20Controller%20BP)) (Utilities|Name|MakeLiteralName "HasLineOfSight"))
    (if (not (Variables|Default|GetisPlayerCaught?))
      (Variables|Default|SetcaughtTime (Utilities|Time|GetTimeSeconds))
      (Variables|Default|SetisPlayerCaught? true))))

(event OnComponentEndOverlap(Capsule)
  (params (OverlappedComponent :type Primitive%20Component%20Object%20Reference) (OtherActor :type Actor%20Object%20Reference) (OtherComp :type Primitive%20Component%20Object%20Reference) (OtherBodyIndex :type Integer))
  (Utilities|Casting|CastToBP_ThirdPersonCharacter OtherActor)
  (if (ScalableFloat|GetValueasBool (Variables|/Script/AIModule.AIController|GetBlackboard (Variables|Default|GetAs%20Dog%20AI%20Controller%20BP)) (Utilities|Name|MakeLiteralName "HasLineOfSight"))
    (Variables|Default|SetisPlayerCaught? false)
    (Variables|Default|SetcaughtTime (Utilities|Time|GetTimeSeconds))))

(event EventBeginPlay
  (bind _asdog_ai_controller_bp (Utilities|Casting|CastToDogAI_Controller_BP (Pawn|GetController)))
  (Variables|Default|SetAs%20Dog%20AI%20Controller%20BP _asdog_ai_controller_bp))

(event EventTick
  (params (DeltaSeconds :type Float%20%28single-precision%29))
  (bind _returnvalue (Game|GetPlayerController 0))
  (if (Variables|Default|GetisPlayerCaught?)
    (if (> (- (Utilities|Time|GetTimeSeconds) (Variables|Default|GetcaughtTime)) (Variables|Default|GettimeToCatch))
      (Input|DisableInput (Pawn|GetControlledPawn _returnvalue) _returnvalue)
      (bind _returnvalue_2 (UserInterface|CreateWidget "/Game/Blueprints/UI/NewWidgetBlueprint.NewWidgetBlueprint_C"))
      (UserInterface|Viewport|AddtoViewport _returnvalue_2 0)
      (Utilities|FlowControl|Delay 2.0)
      (bind _asgame_mode (Utilities|Casting|CastToGameMode (Game|GetGameMode)))
      (Class|GameMode|RestartGame _asgame_mode))))

(fn ConstructionScript)

(fn UpdateWalkSpeed
  (params (NewWalkSpeed :type Float%20%28double-precision%29))
  (Variables|/Script/Engine.CharacterMovementComponent|SetMaxWalkSpeed (Variables|Character|GetCharacterMovement) NewWalkSpeed))