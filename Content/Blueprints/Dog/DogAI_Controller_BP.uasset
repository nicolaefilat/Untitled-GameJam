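; AI controller for the dog, which detects the player wolf by sound and sight and runs a behavior tree on possession.
; Successful perception of a Player-tagged actor feeds two handlers that write to the blackboard.
; Hearing stores the noise location and starts a timed investigation.
; Sight ignores players in sheep form, otherwise setting the enemy and line-of-sight keys and notifying the character it was seen.
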(event OnTargetPerceptionUpdated(AIPerception)
  (params (Actor :type Actor%20Object%20Reference) (Stimulus :type AI%20Stimulus%20Structure))
  (if (and (Actor|ActorHasTag Actor "Player") (.bSuccessfullySensed (Utilities|Struct|BreakAIStimulus Stimulus)))
    (CallFunction|HandleSoundSense Stimulus)
    (CallFunction|HandleVisionSense Stimulus Actor)))

(event Custom|Stop%20Investigation
  (AI|Components|Blackboard|SetValueasBool (Variables|Default|GetBlackboard) (Variables|Default|GetIsInvestigation) false)
  (Development|PrintString "Done Investigation" true true "(R=1.000000,G=0.570049,B=0.206088,A=1.000000)" 2.0 "Investigation"))

(event EventPossess
  (params (PossessedPawn :type Pawn%20Object%20Reference))
  (AI|RunBehaviorTree "/Game/Blueprints/Dog/DogAI_BehaviourTree.DogAI_BehaviourTree"))

(fn ConstructionScript)

(fn HandleSoundSense
  (params (Stimulus :type AI%20Stimulus%20Structure%20%28by%20ref%29))
  (bind _returnvalue (Class|AIPerceptionSystem|GetSenseClassforStimulus Stimulus))
  (if (== _returnvalue "/Script/AIModule.AISense_Hearing")
    (AI|Components|Blackboard|SetValueasVector (Variables|Default|GetBlackboard) (Variables|Default|GetWolfSoundLocationKey) (.StimulusLocation (Utilities|Struct|BreakAIStimulus Stimulus)))
    (AI|Components|Blackboard|SetValueasBool (Variables|Default|GetBlackboard) (Variables|Default|GetIsInvestigation) true)
    (Utilities|Time|SetTimerbyFunctionName 0 "Stop Investigation" (Variables|Default|GetTimeToInvestigate))))

(fn HandleVisionSense
  (params (Stimulus :type AI%20Stimulus%20Structure%20%28by%20ref%29) (Actor :type Actor%20Object%20Reference))
  (bind _blackboard (Variables|Default|GetBlackboard))
  (bind _returnvalue (Class|AIPerceptionSystem|GetSenseClassforStimulus Stimulus))
  (bind _output_get (Variables|Default|SetActor Actor))
  (if (== _returnvalue "/Script/AIModule.AISense_Sight")
    (bind _asbp_third_person_character (Utilities|Casting|CastToBP_ThirdPersonCharacter _output_get))
    (if (not (Variables|/Game/ThirdPerson/Blueprints/BP_ThirdPersonCharacter.BP_ThirdPersonCharacter_C|GetisSheep? _asbp_third_person_character))
      (Utilities|FlowControl|Sequence
        (:then_0
          (AI|Components|Blackboard|SetValueasBool _blackboard (Variables|Default|GetHasLineOfSightKey?) true)
          (AI|Components|Blackboard|SetValueasObject _blackboard (Variables|Default|GetEnemyActorKey) (Variables|Default|GetActor)))
        (:then_1
          (Default|WolfWasSeen _asbp_third_person_character))))))