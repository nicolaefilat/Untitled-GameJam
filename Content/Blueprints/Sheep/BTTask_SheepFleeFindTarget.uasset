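; Behavior tree task for sheep, apparently meant to pick a flee target, but its execute event is empty and never finishes the task.
; Helper functions, none called here, derive navmesh-based candidates from blackboard sphere location and radius.
; The away-from-sphere helper returns an offset rather than a position; Forward and Any variants identically project ahead of the pawn.
; The random-point helper's loop never reaches its return, leaving its angle rotation unused.
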(event EventReceiveExecuteAI
  (params (OwnerController :type AI%20Controller%20Object%20Reference) (ControlledPawn :type Pawn%20Object%20Reference)))

(fn GetNewFleeLocationClosestSphere
  (params (Pawn :type Pawn%20Object%20Reference))
  (return (* (Math|Vector|Normalize (- (Transformation|GetActorLocation Pawn) (.ProjectedLocation (AI|Navigation|ProjectPointtoNavigation (Class|BTFunctionLibrary|GetBlackboardValueasVector (Variables|Default|GetSphereLocationKey)) 0 "/Script/AIModule.NavFilter_AIControllerDefault" "0, 0, 0")))) (Class|BTFunctionLibrary|GetBlackboardValueasFloat (Variables|Default|GetSphereRadiusKey)))))

(fn GetNewFleeLocationRandomSpherefromPosition
  (params (Pawn :type Pawn%20Object%20Reference))
  (Variables|Default|SetdirectionAngle 0.0)
  (while (< (Variables|Default|GetdirectionAngle) 3.6e+02)
    (bind _output_get (Variables|Default|SetdirectionAngle (+ (Variables|Default|GetdirectionAngle) 1e+01)))
    (if (.ReturnValue (AI|Navigation|GetRandomReachablePointinRadius (Transformation|GetActorLocation Pawn) (Class|BTFunctionLibrary|GetBlackboardValueasFloat (Variables|Default|GetSphereRadiusKey)) 0 0))
      _)))

(fn GetNewFreeLocationForwardVector
  (params (Pawn :type Pawn%20Object%20Reference))
  (return (.ProjectedLocation (AI|Navigation|ProjectPointtoNavigation (+ (* (Transformation|GetActorForwardVector Pawn) (Class|BTFunctionLibrary|GetBlackboardValueasFloat (Variables|Default|GetSphereRadiusKey))) (Transformation|GetActorLocation Pawn)) 0 0 "0, 0, 0"))))

(fn GetNewFleeLocationAnyVector
  (params (Pawn :type Pawn%20Object%20Reference))
  (return (.ProjectedLocation (AI|Navigation|ProjectPointtoNavigation (+ (* (Transformation|GetActorForwardVector Pawn) (Class|BTFunctionLibrary|GetBlackboardValueasFloat (Variables|Default|GetSphereRadiusKey))) (Transformation|GetActorLocation Pawn)) 0 0 "0, 0, 0"))))