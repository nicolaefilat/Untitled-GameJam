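; Behavior tree task that picks a random reachable patrol point for a sheep AI and writes it to the blackboard.
; Sheep that have never fled wander within half the radius of their blackboard sphere, falling back to their current position if navigation fails.
; Sheep that have fled patrol around their own location instead.
; A failed search in that branch only prints a message and never finishes the task.
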(event EventReceiveExecuteAI
  (params (OwnerController :type AI%20Controller%20Object%20Reference) (ControlledPawn :type Pawn%20Object%20Reference))
  (bind _spherelocationkey (Variables|Default|GetSphereLocationKey))
  (bind _sphereradiuskey (Variables|Default|GetSphereRadiusKey))
  (bind _returnvalue (Class|BTFunctionLibrary|GetBlackboardValueasVector _spherelocationkey))
  (bind _returnvalue_2 (Class|BTFunctionLibrary|GetBlackboardValueasFloat _sphereradiuskey))
  (bind _returnvalue_3 (/ _returnvalue_2 2.0))
  (bind (_randomlocation _returnvalue_4) (AI|Navigation|GetRandomReachablePointinRadius _returnvalue _returnvalue_3 0 0))
  (bind _output_get (Variables|Default|SetControlled%20Pawn ControlledPawn))
  (Utilities|Casting|CastToSheepAICharacter_BP _output_get
    (:then
      (if (Class|BTFunctionLibrary|GetBlackboardValueasBool (Variables|Default|GetHasEverFledKey))
        ;[0.865 1 0.2145] Fled once
        (if (.ReturnValue (AI|Navigation|GetRandomReachablePointinRadius (Transformation|GetActorLocation (Variables|Default|GetControlled%20Pawn)) (Variables|Default|GetAfterFleePatrolDistance) 0 0))
          (Variables|Default|SetRandom%20Location (.RandomLocation (AI|Navigation|GetRandomReachablePointinRadius (Transformation|GetActorLocation (Variables|Default|GetControlled%20Pawn)) (Variables|Default|GetAfterFleePatrolDistance) 0 0)))
          (AI|BehaviorTree|SetBlackboardValueasVector (Variables|Default|GetPatrolLocation) (Variables|Default|GetRandom%20Location) :!label _label)
          (AI|BehaviorTree|FinishExecute true :!label _label_2)
          (else
            (Development|PrintString "Bad Navigation Can't find" true true "(R=1.000000,G=0.196598,B=0.000000,A=1.000000)")))
        (else
          ;[1 0.2008 0.02672] Has not fled yet. Stick to sphere
          (if _returnvalue_4
            (Variables|Default|SetRandom%20Location _randomlocation)
            (goto _label)
            (else
              (Development|PrintString "failed to find navigation location" true true "(R=1.000000,G=0.117299,B=0.000000,A=1.000000)")
              (AI|BehaviorTree|SetBlackboardValueasVector (Variables|Default|GetPatrolLocation) (Transformation|GetActorLocation (Variables|Default|GetControlled%20Pawn)))
              (goto _label_2))))))
    (:CastFailed
      (AI|BehaviorTree|FinishExecute false))))