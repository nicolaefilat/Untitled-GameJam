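; AI controller for sheep characters that runs the sheep behavior tree when it possesses a pawn.
; A separate InitializeBlackboard event casts the controlled pawn to the sheep character and copies its patrol sphere center and radius into the blackboard.
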(event Custom|Initialize%20Blackboard
  (bind _returnvalue (AI|GetBlackboard 0))
  ;[1 1 1] Setup blackoard items from the sheep character
  (bind _assheep_aicharacter_bp (Utilities|Casting|CastToSheepAICharacter_BP (Pawn|GetControlledPawn)))
  (AI|Components|Blackboard|SetValueasVector _returnvalue (Variables|Default|GetSpherePatrolLocation) (Variables|/Game/Blueprints/Sheep/SheepAICharacter_BP.SheepAICharacter_BP_C|GetPatrolSphereCenter _assheep_aicharacter_bp))
  (AI|Components|Blackboard|SetValueasFloat _returnvalue (Variables|Default|GetSpherePatrolRadius) (Variables|/Game/Blueprints/Sheep/SheepAICharacter_BP.SheepAICharacter_BP_C|GetPatrol%20Radius _assheep_aicharacter_bp)))

(event EventPossess
  (params (PossessedPawn :type Pawn%20Object%20Reference))
  (AI|RunBehaviorTree "/Game/Blueprints/Sheep/SheepAI_BehaviourTree.SheepAI_BehaviourTree"))

(fn ConstructionScript)