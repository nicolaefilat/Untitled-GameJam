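; Behavior tree task that picks the next patrol point for an AI sheep within a sphere area stored on the blackboard.
; It reads the sphere's location and radius keys, finds a random reachable point inside, and writes it to PatrolLocation, falling back to the pawn's current location.
; It only sets the target, succeeds for SheepAICharacter_BP pawns and fails otherwise.
; A debug print outputs the sphere center on each run.
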(event EventReceiveExecuteAI
  (params (OwnerController :type AI%20Controller%20Object%20Reference) (ControlledPawn :type Pawn%20Object%20Reference))
  (bind _spherelocationkey (Variables|Default|GetSphereLocationKey))
  (bind _sphereradiuskey (Variables|Default|GetSphereRadiusKey))
  (bind _returnvalue (Class|BTFunctionLibrary|GetBlackboardValueasVector _spherelocationkey))
  (bind _returnvalue_2 (Class|BTFunctionLibrary|GetBlackboardValueasFloat _sphereradiuskey))
  (bind (_randomlocation _returnvalue_3) (AI|Navigation|GetRandomReachablePointinRadius _returnvalue _returnvalue_2 0 0))
  (Utilities|Casting|CastToSheepAICharacter_BP ControlledPawn
    (:then
      (Development|PrintString (Utilities|String|ToString(Vector) _returnvalue))
      (if _returnvalue_3
        (AI|BehaviorTree|SetBlackboardValueasVector (Variables|Default|GetPatrolLocation) _randomlocation)
        (else
          (AI|BehaviorTree|SetBlackboardValueasVector (Variables|Default|GetPatrolLocation) (Transformation|GetActorLocation ControlledPawn))))
      (AI|BehaviorTree|FinishExecute true))
    (:CastFailed
      (AI|BehaviorTree|FinishExecute false))))