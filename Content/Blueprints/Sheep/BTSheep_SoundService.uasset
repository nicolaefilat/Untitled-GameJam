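; Behavior tree service for sheep AI that plays a sheep sound at the controlled pawn's location at randomized intervals.
; On AI activation it starts a one-shot timer, and each playback uses sound attenuation and schedules the next timer.
; Each delay is the base wait plus a random amount up to the deviation, and no deactivation handler clears the timer.
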(event Custom|PlaySheepSound
  (Audio|PlaySoundatLocation (Variables|Default|GetSound) (Transformation|GetActorLocation (stale EventReceiveActivationAI ControlledPawn)) "0, 0, 0" 1.0 1.0 0.0 "/Game/Sound/NewSoundAttenuation.NewSoundAttenuation" 0 0 0)
  (bind _waittime (CallFunction|GenerateRandomWaitTime))
  (Utilities|Time|SetTimerbyEvent (delegate Custom|PlaySheepSound) _waittime))

(event EventReceiveActivationAI
  (params (OwnerController :type AI%20Controller%20Object%20Reference) (ControlledPawn :type Pawn%20Object%20Reference))
  (bind _waittime (CallFunction|GenerateRandomWaitTime))
  (Utilities|Time|SetTimerbyEvent (delegate Custom|PlaySheepSound) _waittime))

(fn GenerateRandomWaitTime
  (return (+ (Variables|Default|GetplaySoundWait) (Math|Random|RandomFloatinRange 0.0 (Variables|Default|GetrandomWaitDeviation)))))