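; Sheep AI character that patrols a sphere area, can temporarily follow the player, flees when nearby sheep die, and can be killed.
; It takes patrol bounds from an assigned sphere, re-centred on request, and drives SheepAI_Controller_BP through Blackboard keys.
; Following enables a throttled Tick that updates the player's location until a cooldown expires or the player's IsSheep turns false.
; Death flashes red, destroys the actor and notifies the player.
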(event Custom|DieEvent
  ;[1 1 1] Sheep gets killed
  (Rendering|Material|SetMaterial (Variables|Default|GetStaticMesh) 0 "/Game/Materials/ML_Solid_Red.ML_Solid_Red")
  (Utilities|FlowControl|Delay 0.75)
  (Actor|DestroyActor)
  (Default|OneSheepDied (Variables|Default|GetPlayer)))

(event Custom|SheepMovesToPlayer
  (bind _sheepaicontroller (Variables|Default|GetSheepAIController))
  (bind _blackboard (Variables|/Script/AIModule.AIController|GetBlackboard _sheepaicontroller))
  ;[1 0.08646 0.08646] Sheep moves to the player
  (if (not (Variables|Default|GetIsFollowingPlayer?))
    (Variables|Default|SetIsFollowingPlayer? true)
    (Actor|Tick|SetActorTickEnabled true)
    (Actor|Tick|SetActorTickInterval 0.1)
    (AI|Components|Blackboard|SetValueasBool _blackboard (Variables|Default|GetIsFollowingPlayerKey) true)
    (AI|Components|Blackboard|SetValueasVector _blackboard (Variables|Default|GetfollowPlayerLocationKey) (Transformation|GetActorLocation (Variables|Default|GetPlayer)))
    (Development|SetHiddeninGame (Variables|Default|GetSphere) false false)
    (Utilities|FlowControl|Delay (Variables|Default|GetFollowPlayerCooldown))
    (CallFunction|SheepNotFollowPlayer)))

(event Custom|SheepDieInCloseRangeEvent
  (bind _sheepaicontroller (Variables|Default|GetSheepAIController))
  (bind _blackboard (Variables|/Script/AIModule.AIController|GetBlackboard _sheepaicontroller))
  ;[0 0.9859 1] Shep Event to when another sheep dies in close range
  (AI|Components|Blackboard|SetValueasBool _blackboard (Variables|Default|GetisFleeingFromDeadSheepKey) true)
  (Utilities|FlowControl|Delay (Variables|Default|GetSheepDeadBeeCooldown))
  (AI|Components|Blackboard|SetValueasBool _blackboard (Variables|Default|GetisFleeingFromDeadSheepKey) false))

(event Custom|UpdateSphereComponent
  (params (SphereLocation :type Vector))
  ;[1 1 1] Update Sphere Component when wolf comes closer
  (Variables|Default|SetPatrolSphereCenter SphereLocation)
  (bind _assheep_ai_controller_bp (Utilities|Casting|CastToSheepAI_Controller_BP (Pawn|GetController)))
  (Default|InitializeBlackboard _assheep_ai_controller_bp))

(event Custom|SheepNotFollowPlayer
  ;[1 0.08646 0.08646] Sheep moves to the player
  (Variables|Default|SetIsFollowingPlayer? false)
  (Actor|Tick|SetActorTickEnabled false)
  (AI|Components|Blackboard|SetValueasBool (Variables|/Script/AIModule.AIController|GetBlackboard (Variables|Default|GetSheepAIController)) (Variables|Default|GetIsFollowingPlayerKey) false)
  (Development|SetHiddeninGame (Variables|Default|GetSphere) true false))

(event EventTick
  (params (DeltaSeconds :type Float%20%28single-precision%29))
  (bind _player (Variables|Default|GetPlayer))
  ;[1 0.08646 0.08646] Sheep moves to the player
  (if (Variables|Default|GetIsFollowingPlayer?)
    (if (Variables|/Game/ThirdPerson/Blueprints/BP_ThirdPersonCharacter.BP_ThirdPersonCharacter_C|GetisSheep? _player)
      (AI|Components|Blackboard|SetValueasVector (Variables|/Script/AIModule.AIController|GetBlackboard (Variables|Default|GetSheepAIController)) (Variables|Default|GetfollowPlayerLocationKey) (Transformation|GetActorLocation _player))
      (else
        (CallFunction|SheepNotFollowPlayer)))))

(event EventBeginPlay
  (bind _spherecomponent (Variables|Default|GetSphereComponent))
  (bind _returnvalue (Actor|GetComponentbyClass _spherecomponent "/Script/Engine.SphereComponent"))
  ;[1 1 1] Get the radius and location from the Sphere Component that was attached
  (Utilities|FlowControl|Sequence
    (:then_0
      (if (Utilities|IsValid (Variables|Default|GetSphereComponent))
        (Variables|Default|SetPatrol%20Radius (Components|Sphere|GetScaledSphereRadius _returnvalue))
        (Variables|Default|SetPatrolSphereCenter (Transformation|GetWorldLocation _returnvalue))
        (bind _assheep_ai_controller_bp (Utilities|Casting|CastToSheepAI_Controller_BP (Pawn|GetController))
          (:then
            (Default|InitializeBlackboard _assheep_ai_controller_bp))
          (:CastFailed
            (Development|PrintString "Cast failed !!" true true "(R=1.000000,G=0.013872,B=0.000000,A=1.000000)")))
        (else
          (Development|PrintString (Utilities|String|Append "The sheep" (Utilities|GetDisplayName (Components|GetOwner)) "is not in a sphere box component. It won't work!!!. 
Make sure the sheep is inside a ShapeBox_BP component!") true true "(R=1.000000,G=0.000000,B=0.035222,A=1.000000)" 1e+03))))
    (:then_1
      ;[1 1 1] Set SheepControllerAI
      (bind _assheep_ai_controller_bp_2 (Utilities|Casting|CastToSheepAI_Controller_BP (Pawn|GetController)))
      (Variables|Default|SetSheepAIController _assheep_ai_controller_bp_2))
    (:then_2
      (bind _asbp_third_person_character (Utilities|Casting|CastToBP_ThirdPersonCharacter (Game|Player|GetPlayerPawn 0)))
      (Variables|Default|SetPlayer _asbp_third_person_character))))

(fn ConstructionScript)